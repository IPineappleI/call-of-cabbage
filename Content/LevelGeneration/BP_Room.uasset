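; Procedurally generated level room that builds itself on BeginPlay, sized and populated by difficulty and the game instance's seeded random stream.
; Advances the room counter, offsets itself to the entry door, then lays instanced floors and walls.
; Scatters traps, buffs, debuffs and items, using self-adjusting probabilities for moving traps and effects.
; Non-final rooms get two linked exit doors; hard rooms raise difficulty and add healing; the last holds the cabbage pile.
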(event EventBeginPlay
  (CallFunction|InitializeVariables)
  (CallFunction|OffsetRoom)
  (CallFunction|BuildRoom))

(event Collision|EventActorBeginOverlap
  (params (OtherActor :type Actor%20Object%20Reference)))

(event EventTick
  (params (DeltaSeconds :type Float%20%28single-precision%29)))

(fn ConstructionScript
  ;[1 1 1] Connect for in-editor testing
)

(fn BuildRoom
  (CallFunction|BuildFloorandStuff)
  (CallFunction|BuildWallsandDoors)
  ;[1 1 1] Spawn a healing item
  (if (Variables|Default|GetIsHard)
    (Game|SpawnActorfromClass "/Game/LevelGeneration/BP_HealingItem.BP_HealingItem_C" (Math|Transform|MakeTransform (+ (Transformation|GetActorLocation) (Math|Vector|MakeVector (Variables|Default|GetXTileSize) (* (Variables|Default|GetYTileSize) (/ (Variables|Default|GetYTilesCount) 2)) 0.0)) "0, 0, 0" "1.000000,1.000000,1.000000") "Undefined" "MultiplyWithRoot" 0 0))
  ;[1 1 1] Spawn the cabbage pile
  (if (Variables|Default|GetIsTheLastRoom)
    (Game|SpawnActorfromClass "/Game/LevelGeneration/BP_CabbagePile.BP_CabbagePile_C" (Math|Transform|MakeTransform (+ (Transformation|GetActorLocation) (Math|Vector|MakeVector (* (Variables|Default|GetXTileSize) (- (Variables|Default|GetXTilesCount) 1)) (* (Variables|Default|GetYTileSize) (/ (Variables|Default|GetYTilesCount) 2)) 0.0)) "0, 0, 0" "1.000000,1.000000,1.000000") "Undefined" "MultiplyWithRoot" 0 0)))

(fn BuildFloorandStuff
  (bind _returnvalue (Transformation|GetActorLocation))
  (bind _xtilescount (Variables|Default|GetXTilesCount))
  (bind _xtilesize (Variables|Default|GetXTileSize))
  (bind _gameinstance (Variables|Default|GetGameInstance))
  (bind _random (Variables|/Game/LevelGeneration/BP_CabbageInstance.BP_CabbageInstance_C|GetRandom _gameinstance))
  ;[1 1 1] Build the floor of the room
  (for _index (range 0 (- _xtilescount 1))
    (for _index_2 (range 0 (- (Variables|Default|GetYTilesCount) 1))
      (Components|InstancedStaticMesh|AddInstance (Variables|Default|GetFloor) (Math|Transform|MakeTransform (Math|Vector|MakeVector (* _index (Variables|Default|GetXTileSize)) (* _index_2 (Variables|Default|GetYTileSize)) 0.0) "0, 0, 0" "1.000000,1.000000,1.000000") false)
      ;[1 1 1] Place spike traps
      (if (and (> _index 1) (< _index (- _xtilescount 2)))
        (Utilities|FlowControl|Sequence
          (:then_0
            ;[1 1 1] Place moving traps
            (if (== _index_2 0)
              (if (Class|KismetMathLibrary|RandomBoolwithWeightfromStream (Variables|/Game/LevelGeneration/BP_CabbageInstance.BP_CabbageInstance_C|GetRandom (Variables|Default|GetGameInstance)) (LocalVariables|GetMovingTrapProbability))
                (Game|SpawnActorfromClass "/Game/LevelGeneration/BP_MovingTrap.BP_MovingTrap_C" (Math|Transform|MakeTransform (+ (Math|Vector|MakeVector (+ (+ (* _index (Variables|Default|GetXTileSize)) (.x _returnvalue)) 2e+02) (+ (+ (* _index_2 (Variables|Default|GetYTileSize)) (.y _returnvalue)) 2e+02) 0.0) "0.000000,0.000000,69.000000") "0, 0, 0" "1.000000,1.000000,1.000000") "Undefined" "MultiplyWithRoot" 0 (Math|Vector|MakeVector (- (* (Math|Random|RandomIntegerinRangefromStream (Variables|/Game/LevelGeneration/BP_CabbageInstance.BP_CabbageInstance_C|GetRandom (Variables|Default|GetGameInstance)) 2 (- (Variables|Default|GetXTilesCount) 3)) _xtilesize) (* _xtilesize _index)) (* (- (Variables|Default|GetYTilesCount) 1) (Variables|Default|GetYTileSize)) 0.0) 0)
                (LocalVariables|SetMovingTrapProbability (Math|Float|Clamp(Float) (- (LocalVariables|GetMovingTrapProbability) (- 0.5 (* (Variables|Default|GetDifficulty) 0.02)))))
                (else
                  (LocalVariables|SetMovingTrapProbability (Math|Float|Clamp(Float) (+ (LocalVariables|GetMovingTrapProbability) (+ 0.25 (* (Variables|Default|GetDifficulty) 0.01)))))))))
          (:then_1
            (if (Class|KismetMathLibrary|RandomBoolwithWeightfromStream (Variables|/Game/LevelGeneration/BP_CabbageInstance.BP_CabbageInstance_C|GetRandom (Variables|Default|GetGameInstance)) (+ 0.4 (* (Variables|Default|GetDifficulty) 0.02)))
              (Game|SpawnActorfromClass "/Game/LevelGeneration/BP_SpikeTrap.BP_SpikeTrap_C" (Math|Transform|MakeTransform (Math|Vector|MakeVector (+ (+ (* _index (Variables|Default|GetXTileSize)) (.x _returnvalue)) 2e+02) (+ (+ (* _index_2 (Variables|Default|GetYTileSize)) (.y _returnvalue)) 2e+02) 0.0) "0, 0, 0" "1.000000,1.000000,1.000000") "Undefined" "MultiplyWithRoot" 0 0)))
          (:then_2
            ;[1 1 1] Spawn buffs
            (if (Class|KismetMathLibrary|RandomBoolwithWeightfromStream _random (Math|Float|Clamp(Float) (- (LocalVariables|GetBuffProbability) (* (Variables|Default|GetDifficulty) 0.02))))
              (if (Math|Random|RandomBoolfromStream _random)
                (Game|SpawnActorfromClass "/Game/LevelGeneration/BP_SlowTrapsBuff.BP_SlowTrapsBuff_C" (Math|Transform|MakeTransform (Math|Vector|MakeVector (+ (+ (* _index (Variables|Default|GetXTileSize)) (.x _returnvalue)) 2e+02) (+ (+ (* _index_2 (Variables|Default|GetYTileSize)) (.y _returnvalue)) 2e+02) 0.0) "0, 0, 0" "1.000000,1.000000,1.000000") "Undefined" "MultiplyWithRoot" 0 0)
                (else
                  (Game|SpawnActorfromClass "/Game/LevelGeneration/BP_SpikeImmunityBuff.BP_SpikeImmunityBuff_C" (Math|Transform|MakeTransform (Math|Vector|MakeVector (+ (+ (* _index (Variables|Default|GetXTileSize)) (.x _returnvalue)) 2e+02) (+ (+ (* _index_2 (Variables|Default|GetYTileSize)) (.y _returnvalue)) 2e+02) 0.0) "0, 0, 0" "1.000000,1.000000,1.000000") "Undefined" "MultiplyWithRoot" 0 0)))
              (LocalVariables|SetBuffProbability 0.0)
              (else
                (LocalVariables|SetBuffProbability (Math|Float|Clamp(Float) (+ (LocalVariables|GetBuffProbability) 0.02)))
                ;[1 1 1] Spawn debuffs
                (if (Class|KismetMathLibrary|RandomBoolwithWeightfromStream (Variables|/Game/LevelGeneration/BP_CabbageInstance.BP_CabbageInstance_C|GetRandom (Variables|Default|GetGameInstance)) (Math|Float|Clamp(Float) (+ (LocalVariables|GetDebuffProbability) (* (Variables|Default|GetDifficulty) 0.02))))
                  (Game|SpawnActorfromClass "/Game/LevelGeneration/BP_SlowdownDebuff.BP_SlowdownDebuff_C" (Math|Transform|MakeTransform (Math|Vector|MakeVector (+ (+ (* _index (Variables|Default|GetXTileSize)) (.x _returnvalue)) 2e+02) (+ (+ (* _index_2 (Variables|Default|GetYTileSize)) (.y _returnvalue)) 2e+02) 0.0) "0, 0, 0" "1.000000,1.000000,1.000000") "Undefined" "MultiplyWithRoot" 0 0)
                  (LocalVariables|SetDebuffProbability 0.0)
                  (else
                    (LocalVariables|SetDebuffProbability (Math|Float|Clamp(Float) (+ (LocalVariables|GetDebuffProbability) 0.02)))
                    ;[1 1 1] Spawn random items
                    (if (Class|KismetMathLibrary|RandomBoolwithWeightfromStream (Variables|/Game/LevelGeneration/BP_CabbageInstance.BP_CabbageInstance_C|GetRandom (Variables|Default|GetGameInstance)) 0.05)
                      (Game|SpawnActorfromClass "/Game/LevelGeneration/BP_RandomItem.BP_RandomItem_C" (Math|Transform|MakeTransform (Math|Vector|MakeVector (+ (+ (* _index (Variables|Default|GetXTileSize)) (.x _returnvalue)) 2e+02) (+ (+ (* _index_2 (Variables|Default|GetYTileSize)) (.y _returnvalue)) 2e+02) 0.0) "0, 0, 0" "1.000000,1.000000,1.000000") "Undefined" "MultiplyWithRoot" 0 0))))))))))))

(fn BuildWallsandDoors
  (bind _returnvalue (Transformation|GetActorLocation))
  (bind _ishard (Variables|Default|GetIsHard))
  (bind _ytilescount (Variables|Default|GetYTilesCount))
  (bind _returnvalue_2 (- _ytilescount 1))
  ;[1 1 1] Build the X-parallel walls
  (for _index (range 0 (- (Variables|Default|GetXTilesCount) 1))
    (Components|InstancedStaticMesh|AddInstance (Variables|Default|GetWall) (Math|Transform|MakeTransform (Math|Vector|MakeVector (* _index (Variables|Default|GetXTileSize)) 0.0 0.0) "0, 0, 0" "1.000000,1.000000,1.000000") false)
    (Components|InstancedStaticMesh|AddInstance (Variables|Default|GetWall) (Math|Transform|MakeTransform (Math|Vector|MakeVector (* _index (Variables|Default|GetXTileSize)) (* (Variables|Default|GetYTilesCount) (Variables|Default|GetYTileSize)) 0.0) "0, 0, 0" "1.000000,1.000000,1.000000") false))
  ;[1 1 1] Build the Y-parallel walls, the doors and the gaps
  (for _index_2 (range 0 _returnvalue_2)
    (if (and (not (Variables|Default|GetIsTheFirstRoom)) (or (and (not _ishard) (== _index_2 (- _returnvalue_2 1))) (and _ishard (== _index_2 1)))) ; True - gap, False - Wall
      _
      (else
        (Components|InstancedStaticMesh|AddInstance (Variables|Default|GetWall) (Math|Transform|MakeTransform (Math|Vector|MakeVector 0.0 (* _index_2 (Variables|Default|GetYTileSize)) 0.0) "0.000000,90.000000,0.000000" "1.000000,1.000000,1.000000") false)))
    (if (and (or (== _index_2 1) (== _index_2 (- _returnvalue_2 1))) (not (Variables|Default|GetIsTheLastRoom))) ; True - Door, False - Wall
      (bind _returnvalue_3 (Game|SpawnActorfromClass "/Game/LevelGeneration/BP_Door.BP_Door_C" (Math|Transform|MakeTransform (Math|Vector|MakeVector (+ (.X (Math|Vector|BreakVector (Math|Vector|MakeVector (* (Variables|Default|GetXTilesCount) (Variables|Default|GetXTileSize)) (* _index_2 (Variables|Default|GetYTileSize)) 0.0))) (.x _returnvalue)) (+ (+ (.Y (Math|Vector|BreakVector (Math|Vector|MakeVector (* (Variables|Default|GetXTilesCount) (Variables|Default|GetXTileSize)) (* _index_2 (Variables|Default|GetYTileSize)) 0.0))) (Variables|Default|GetYTileSize)) (.y _returnvalue)) 0.0) "0.000000,-90.000000,0.000000" "1.000000,1.000000,1.000000") "Undefined" "MultiplyWithRoot" 0 (== _index_2 (- _returnvalue_2 1)) 0))
      (if (== _index_2 (- _returnvalue_2 1))
        (LocalVariables|SetRightDoor _returnvalue_3)
        (else
          (LocalVariables|SetLeftDoor _returnvalue_3)))
      (else
        (Components|InstancedStaticMesh|AddInstance (Variables|Default|GetWall) (Math|Transform|MakeTransform (Math|Vector|MakeVector (* (Variables|Default|GetXTilesCount) (Variables|Default|GetXTileSize)) (* _index_2 (Variables|Default|GetYTileSize)) 0.0) "0.000000,90.000000,0.000000" "1.000000,1.000000,1.000000") false))))
  ;[1 1 1] Give the left and the right doors references of each other
  (if (not (Variables|Default|GetIsTheLastRoom))
    (Variables|/Game/LevelGeneration/BP_Door.BP_Door_C|SetOtherDoor (LocalVariables|GetLeftDoor) (LocalVariables|GetRightDoor))
    (Variables|/Game/LevelGeneration/BP_Door.BP_Door_C|SetOtherDoor (LocalVariables|GetRightDoor) (LocalVariables|GetLeftDoor))))

(fn OffsetRoom
  ;[1 1 1] Offset the room for the door
  (if (not (Variables|Default|GetIsTheFirstRoom))
    (if (not (Variables|Default|GetIsHard))
      (Transformation|AddLocalOffset (Variables|Default|GetDefaultSceneRoot) (Math|Vector|MakeVector 0.0 (* (Variables|Default|GetYTileSize) (* (- (Variables|Default|GetYTilesCount) 1) -1.0)) 0.0) false false)
      (else
        (Transformation|AddLocalOffset (Variables|Default|GetDefaultSceneRoot) (Math|Vector|MakeVector 0.0 (* (Variables|Default|GetYTileSize) -2.0) 0.0) false false)))))

(fn InitializeVariables
  ;[1 1 1] Initialize variables based on game instance
  (bind _asbp_cabbage_instance (Utilities|Casting|CastToBP_CabbageInstance (Game|GetGameInstance)))
  (bind _output_get (Variables|Default|SetGameInstance _asbp_cabbage_instance))
  (bind _output_get_2 (Variables|/Game/LevelGeneration/BP_CabbageInstance.BP_CabbageInstance_C|SetCurrentRoom _asbp_cabbage_instance (+ (Variables|/Game/LevelGeneration/BP_CabbageInstance.BP_CabbageInstance_C|GetCurrentRoom _output_get) 1)))
  (if (== _output_get_2 1)
    (Variables|Default|SetIsTheFirstRoom true))
  (if (== _output_get_2 (Variables|/Game/LevelGeneration/BP_CabbageInstance.BP_CabbageInstance_C|GetTotalRooms _asbp_cabbage_instance))
    (Variables|Default|SetIsTheLastRoom true))
  (if (Variables|Default|GetIsHard)
    (bind _output_get_3 (Variables|/Game/LevelGeneration/BP_CabbageInstance.BP_CabbageInstance_C|SetDifficulty (Variables|Default|GetGameInstance) (+ (Variables|/Game/LevelGeneration/BP_CabbageInstance.BP_CabbageInstance_C|GetDifficulty (Variables|Default|GetGameInstance)) 1)))
    (Variables|Default|SetDifficulty _output_get_3)
    (else
      (Variables|Default|SetDifficulty (Variables|/Game/LevelGeneration/BP_CabbageInstance.BP_CabbageInstance_C|GetDifficulty (Variables|Default|GetGameInstance)))))
  (Variables|Default|SetXTilesCount (Math|Random|RandomIntegerinRangefromStream (Variables|/Game/LevelGeneration/BP_CabbageInstance.BP_CabbageInstance_C|GetRandom (Variables|Default|GetGameInstance)) (+ (/ (Variables|Default|GetDifficulty) 3) 9) (+ (/ (Variables|Default|GetDifficulty) 2) 9)))
  (Variables|Default|SetYTilesCount (Math|Random|RandomIntegerinRangefromStream (Variables|/Game/LevelGeneration/BP_CabbageInstance.BP_CabbageInstance_C|GetRandom (Variables|Default|GetGameInstance)) (+ (/ (Variables|Default|GetDifficulty) 3) 5) (+ (/ (Variables|Default|GetDifficulty) 2) 5))))