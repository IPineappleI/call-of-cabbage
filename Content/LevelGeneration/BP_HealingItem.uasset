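; BP_HealingItem is a pickup that heals the player character on overlap, then destroys itself.
; On BeginPlay it reads its healing amount from the Cabbage settings and starts a Floating timeline that updates the Sphere's relative height and yaw.
; Only BP_ThirdPersonCharacter triggers the pickup, and healing is delivered through ApplyDamage as negative damage rather than a separate heal function.
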(event EventBeginPlay
  ;[1 1 1] Initialize the healing variable and the floating animation
  (bind _returnvalue (Class|CabbageSettings|GetCabbageSettings))
  (Variables|Default|SetHealing (Class|CabbageSettings|GetHealing _returnvalue))
  (bind (_direction _z _yaw) (Timeline|Floating Play)
    (:Update
      (Transformation|SetRelativeTransform (Variables|Default|GetSphere) (Math|Transform|MakeTransform (Math|Vector|MakeVector 0.0 0.0 _z) (Math|Rotator|MakeRotator 0.0 0.0 _yaw) "1.000000,1.000000,1.000000") false false))))

(event Collision|EventActorBeginOverlap
  (params (OtherActor :type Actor%20Object%20Reference))
  ;[1 1 1] Heal the player (apply negative damage) and self-destroy
  (bind _asbp_third_person_character (Utilities|Casting|CastToBP_ThirdPersonCharacter OtherActor))
  (bind _result (Math|Float|NegateFloat (Variables|Default|GetHealing))
    (:%20%20
      (Game|Damage|ApplyDamage _asbp_third_person_character _result 0 0)
      (Actor|DestroyActor))))

(fn ConstructionScript)