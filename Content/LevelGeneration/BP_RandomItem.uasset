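; Mystery pickup that grants a random effect when the third-person character overlaps it, then destroys itself.
; From BeginPlay, a self-calling Animation event with delays endlessly cycles visibility between the green cylinder, red cylinder and cone meshes.
; On overlap, the Cabbage game instance's random stream picks between triggering SlowTraps on that instance, slowing the character, or making it spike immune.
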(event Custom|Animation
  ;[1 1 1] Loop animation
  (Utilities|FlowControl|Delay 0.25)
  (Development|SetHiddeninGame (Variables|Default|GetGreenCylinder) true false)
  (Development|SetHiddeninGame (Variables|Default|GetRedCylinder) false false)
  (Utilities|FlowControl|Delay 0.25)
  (Development|SetHiddeninGame (Variables|Default|GetRedCylinder) true false)
  (Development|SetHiddeninGame (Variables|Default|GetCone) false false)
  (Utilities|FlowControl|Delay 0.25)
  (Development|SetHiddeninGame (Variables|Default|GetCone) true false)
  (Development|SetHiddeninGame (Variables|Default|GetGreenCylinder) false false)
  (CallFunction|Animation))

(event EventBeginPlay
  ;[1 1 1] Loop animation
  (CallFunction|Animation))

(event Collision|EventActorBeginOverlap
  (params (OtherActor :type Actor%20Object%20Reference))
  ;[1 1 1] Apply random effect
  (bind _asbp_third_person_character (Utilities|Casting|CastToBP_ThirdPersonCharacter OtherActor))
  (bind _asbp_cabbage_instance (Utilities|Casting|CastToBP_CabbageInstance (Game|GetGameInstance)))
  (switch int (Math|Random|RandomIntegerinRangefromStream (Variables|/Game/LevelGeneration/BP_CabbageInstance.BP_CabbageInstance_C|GetRandom _asbp_cabbage_instance) 0 2)
    (:0
      (Default|CallSlowTraps _asbp_cabbage_instance))
    (:1
      (Default|SlowDown _asbp_third_person_character))
    (:2
      (Default|BecomeSpikeImmune _asbp_third_person_character)))
  (Actor|DestroyActor))

(fn ConstructionScript)