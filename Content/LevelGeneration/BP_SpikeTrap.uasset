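; Spike trap actor that damages the player character when it begins overlapping the trap.
; On BeginPlay it builds a square grid of scaled-down spikes as instances of the Spike component.
; The damage amount comes from the Cabbage settings, re-read inside the spawn loop for every instance.
; Overlaps from actors other than BP_ThirdPersonCharacter are ignored, and damage is applied once per overlap begin.
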(event EventBeginPlay
  ;[1 1 1] Spawn the spikes
  (for _index (range 0 9)
    (for _index_2 (range 0 9)
      (Components|InstancedStaticMesh|AddInstance (Variables|Default|GetSpike) (Math|Transform|MakeTransform (Math|Vector|MakeVector (Math|Conversions|ToFloat(Integer) (* _index 20)) (Math|Conversions|ToFloat(Integer) (* _index_2 20)) 0.0) "0, 0, 0" "0.200000,0.200000,0.200000") false)
      ;[1 1 1] Initialize damage variable according to config
      (bind _returnvalue (Class|CabbageSettings|GetCabbageSettings))
      (Variables|Default|SetDamage (Class|CabbageSettings|GetSpikeTrapDamage _returnvalue)))))

(event Collision|EventActorBeginOverlap
  (params (OtherActor :type Actor%20Object%20Reference))
  ;[1 1 1] Apply damage to player
  (bind _asbp_third_person_character (Utilities|Casting|CastToBP_ThirdPersonCharacter OtherActor))
  (Game|Damage|ApplyDamage _asbp_third_person_character (Variables|Default|GetDamage) 0 self))

(event EventTick
  (params (DeltaSeconds :type Float%20%28single-precision%29)))

(fn ConstructionScript)