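; Moving trap for level generation that damages the player character on overlap, with damage and speed read from Cabbage settings.
; A timeline slides its Sphere along RelativeVector from a random start time drawn from the game instance's seeded stream.
; Play rate scales with the vector's Y share of its length.
; The game instance's SlowTraps event halves the speed until a timer restores it, sooner at higher difficulty.
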(event Custom|SlowDown
  ;[1 1 1] React to Slow Traps Buff
  (Components|Timeline|SetPlayRate (Variables|Default|GetMovement) (* (* (Class|CabbageSettings|GetTrapSpeed (stale EventBeginPlay _returnvalue_2)) (/ (.y (Variables|Default|GetRelativeVector)) (Math|Vector|VectorLength (Variables|Default|GetRelativeVector)))) 0.5))
  (bind _asbp_cabbage_instance (Utilities|Casting|CastToBP_CabbageInstance (Game|GetGameInstance)))
  (Utilities|Time|SetTimerbyEvent (delegate Custom|SpeedBackUp) (- 5.0 (* (Variables|/Game/LevelGeneration/BP_CabbageInstance.BP_CabbageInstance_C|GetDifficulty _asbp_cabbage_instance) 0.2))))

(event Custom|SpeedBackUp
  ;[1 1 1] React to Slow Traps Buff
  (Components|Timeline|SetPlayRate (Variables|Default|GetMovement) (* (Class|CabbageSettings|GetTrapSpeed (stale EventBeginPlay _returnvalue_2)) (/ (.y (Variables|Default|GetRelativeVector)) (Math|Vector|VectorLength (Variables|Default|GetRelativeVector))))))

(event EventBeginPlay
  ;[1 1 1] Initialize damage variable according to config
  (bind _returnvalue (Class|CabbageSettings|GetCabbageSettings))
  (Variables|Default|SetDamage (Class|CabbageSettings|GetMovingTrapDamage _returnvalue))
  ;[1 1 1] Start looping movement from a random point
  (Utilities|FlowControl|Sequence
    (:then_0
      ;[1 1 1] Scale the movement speed
      (bind _returnvalue_2 (Class|CabbageSettings|GetCabbageSettings))
      (Components|Timeline|SetPlayRate (Variables|Default|GetMovement) (* (Class|CabbageSettings|GetTrapSpeed _returnvalue_2) (/ (.y (Variables|Default|GetRelativeVector)) (Math|Vector|VectorLength (Variables|Default|GetRelativeVector)))))
      (bind _asbp_cabbage_instance (Utilities|Casting|CastToBP_CabbageInstance (Game|GetGameInstance)))
      ;[1 1 1] React to Slow Traps Buff
      (EventDispatchers|BindEventtoSlowTraps _asbp_cabbage_instance (delegate Custom|SlowDown)))
    (:then_1
      (bind _asbp_cabbage_instance_2 (Utilities|Casting|CastToBP_CabbageInstance (Game|GetGameInstance)))
      (bind _floattrack (Timeline|Movement SetNewTime)
        (:Update
          (Transformation|SetRelativeLocation (Variables|Default|GetSphere) (* (Variables|Default|GetRelativeVector) _floattrack) false false))))
    (:then_2
      (Timeline|Movement Play))))

(event Collision|EventActorBeginOverlap
  (params (OtherActor :type Actor%20Object%20Reference))
  ;[1 1 1] Apply damage to player
  (bind _asbp_third_person_character (Utilities|Casting|CastToBP_ThirdPersonCharacter OtherActor))
  (Game|Damage|ApplyDamage _asbp_third_person_character (Variables|Default|GetDamage) 0 0))

(fn ConstructionScript)