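; BP_Door is a level-generation door that spawns a new BP_Room when used, painted red at BeginPlay when IsRed is set.
; Use locks both this door and its paired OtherDoor, spawns the room at the door's location with IsHard taken from IsRed, and plays the Opening timeline to yaw the Hinge.
; Close reverses that timeline.
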(event Custom|CreateNewRoom
  ;[1 1 1] Spawn a new room
  (Game|SpawnActorfromClass "/Game/LevelGeneration/BP_Room.BP_Room_C" (Math|Transform|MakeTransform (Transformation|GetActorLocation) "0, 0, 0" "1.000000,1.000000,1.000000") "Undefined" "MultiplyWithRoot" 0 (Variables|Default|GetIsRed) 0))

(event Custom|Close
  ;[1 1 1] Open and close the door
  (bind _dooryaw (Timeline|Opening Reverse)
    (:Update
      (Transformation|SetRelativeRotation (Variables|Default|GetHinge) (Math|Rotator|MakeRotator 0.0 0.0 _dooryaw) false false))))

(event EventBeginPlay
  ;[1 1 1] Paint the door red
  (if (Variables|Default|GetIsRed)
    (Rendering|Material|SetMaterial (Variables|Default|GetDoor) 1 "/Game/StarterContent/Materials/M_RedDoor.M_RedDoor")))

(event EventTick
  (params (DeltaSeconds :type Float%20%28single-precision%29)))

(event EventUse
  ;[1 1 1] Open and close the door
  (if (Variables|Default|GetIsUseable)
    (Variables|Default|SetIsUseable false)
    (Variables|BP_Door_C|SetIsUseable (Variables|Default|GetOtherDoor) false)
    (CallFunction|CreateNewRoom)
    (bind _dooryaw (Timeline|Opening Play)
      (:Update
        (Transformation|SetRelativeRotation (Variables|Default|GetHinge) (Math|Rotator|MakeRotator 0.0 0.0 _dooryaw) false false)))))

(fn ConstructionScript)